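; BP_Old_WindTurbine is an old wind turbine prop with an optionally animated spinning rotor.
; The construction script yaws the motor housing, pitches the three blades and can toggle the two logo decals' visibility.
; When Animated is set, Tick accumulates RotorSpeed into the rotor's relative roll, offset by RotationDelay.
; The spin is frame-rate dependent because the per-tick increment ignores delta time.
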(event EventBeginPlay)

(event Collision|EventActorBeginOverlap
  (params (OtherActor :type Actor%20Object%20Reference)))

(event EventTick
  (params (DeltaSeconds :type Float%20%28single-precision%29))
  (if (Variables|Default|GetAnimated?)
    (Variables|Default|SetRotator%20Value (+ (Variables|Default|GetRotator%20Value) (Variables|Default|GetRotor%20Speed)))
    (Transformation|SetRelativeRotation (Variables|Default|GetSM_Old_WindTurbine_Rotor) (Math|Rotator|MakeRotator (+ (+ (Variables|Default|GetRotator%20Value) (Variables|Default|GetRotor%20Speed)) (Variables|Default|GetRotation%20Delay)) 0.0 0.0) false false)))

(fn ConstructionScript
  (Transformation|SetRelativeRotation (Variables|Default|GetSM_Old_WindTurbine_Motor_Housing) (Math|Rotator|MakeRotator 0.0 0.0 (Variables|Default|GetMotor%20Rotation)) false false)
  (Transformation|AddLocalRotation (Variables|Default|GetSM_Old_WindTurbine_Blade_1) (Math|Rotator|MakeRotator 0.0 (Variables|Default|GetBlades%20Rotation) 0.0) false false)
  (if (Variables|Default|GetRemove%20Logo?)
    (Rendering|ToggleVisibility (Variables|Default|GetDecal) false)))